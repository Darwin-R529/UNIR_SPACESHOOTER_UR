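; Spawner actor that periodically creates extra-life pickups (BP_ExtraLife) at random spawn points.
; On BeginPlay it starts a looping timer at SpawnTime intervals, which calls SpawnLife on each tick of the timer.
; SpawnLife picks a random scene component on this actor tagged "SpawnPoint" and spawns the pickup at its world transform, adjusting for collisions but always spawning.
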(event Custom|Spawn
  (CallFunction|SpawnLife))

(event EventBeginPlay
  (Utilities|Time|SetTimerbyEvent (delegate Custom|Spawn) (Variables|Default|GetSpawnTime) true))

(event Collision|EventActorBeginOverlap
  (params (OtherActor :type Actor%20Object%20Reference)))

(event EventTick
  (params (DeltaSeconds :type Float%20%28single-precision%29)))

(fn ConstructionScript)

(fn SpawnLife
  (bind _returnvalue (Actor|GetComponentsbyTag "/Script/Engine.SceneComponent" "SpawnPoint"))
  (bind _returnvalue_2 (Game|SpawnActorfromClass "/Game/Players/BP_ExtraLife.BP_ExtraLife_C" (Transformation|GetWorldTransform (Utilities|Array|Get(acopy) _returnvalue (Math|Random|RandomInteger (Utilities|Array|Length _returnvalue)))) "AdjustIfPossibleButAlwaysSpawn" "MultiplyWithRoot" 0 0))
  (return _returnvalue_2))