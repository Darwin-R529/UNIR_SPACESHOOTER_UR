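; BP_PowerUp is a moving pickup that players collect by overlapping it.
; On BeginPlay it caches its forward vector, then moves along it every Tick at Speed without sweeping.
; Overlap with a "Player"-tagged BP_SpaceSCharacter calls NoPowerUp on that character and fires the PlayerGetIt dispatcher.
; The pickup binds to its own dispatcher to destroy itself after a short delay.
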(event Custom|Destroyed_Event
  (Utilities|FlowControl|Delay 0.1)
  (Actor|DestroyActor))

(event EventBeginPlay
  (Variables|Default|SetMovementVector (Transformation|GetActorForwardVector))
  (EventDispatchers|BindEventtoPlayerGetIt (delegate Custom|Destroyed_Event)))

(event Collision|EventActorBeginOverlap
  (params (OtherActor :type Actor%20Object%20Reference))
  (if (Actor|ActorHasTag OtherActor "Player")
    (bind _asbp_space_scharacter (Utilities|Casting|CastToBP_SpaceSCharacter OtherActor))
    (Default|NoPowerUp _asbp_space_scharacter)
    (Default|CallPlayerGetIt)))

(event EventTick
  (params (DeltaSeconds :type Float%20%28single-precision%29))
  (CallFunction|Move DeltaSeconds))

(fn ConstructionScript)

(fn Move
  (params (Delta%20Time :type Float%20%28double-precision%29))
  (Transformation|SetActorLocation (+ (Transformation|GetActorLocation) (* (* Delta%20Time (Variables|Default|GetSpeed)) (Variables|Default|GetMovementVector))) false false))