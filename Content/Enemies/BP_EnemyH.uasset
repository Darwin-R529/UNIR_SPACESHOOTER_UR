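; BP_EnemyH is a child enemy Blueprint that moves sideways and fires in repeating bursts.
; BeginPlay starts a self-retriggering burst loop calling the parent Fire, spaced by interval and cooldown delays.
; Tick calls Move, while overlaps with "Lateral"-tagged actors toggle direction and lower DelayShoot on alternate bounces.
; A separate EnemyShootV2 event, not called here, spawns Ammo at FirePoint with sound.
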(event Custom|EnemyShootV2
  (for _index (range 0 2)
    (bind _returnvalue (Game|SpawnActorfromClass (Variables|Default|GetAmmo) (Transformation|GetWorldTransform (Variables|Default|GetFire%20Point)) "Undefined" "MultiplyWithRoot" 0 0))
    (Transformation|SetActorRotation _returnvalue (Transformation|GetActorRotation))
    (Audio|PlaySound2D "/Game/OSDT/EnemyShoot.EnemyShoot" 1.0 1.0 0.0 0 0)
    (Utilities|FlowControl|Delay 1.0)))

(event Custom|FireBurst
  (Variables|Default|SetBurstIndex 0)
  (CallFunction|FireBurstStep))

(event Custom|FireBurstStep
  (CallFunction|Fire)
  (bind _result (Math|Integer|IncrementInt (Variables|Default|GetBurstIndex))
    (:%20%20
      (if (< _result (Variables|Default|GetBurstCount))
        (Utilities|FlowControl|Delay (Variables|Default|GetBurstInterval))
        (CallFunction|FireBurstStep)
        (else
          (Utilities|FlowControl|Delay (Variables|Default|GetBurstCooldown))
          (CallFunction|FireBurst))))))

(event EventBeginPlay
  (|CallParentFunction)
  (Variables|Default|SetMovementVector (Transformation|GetActorRightVector))
  (Variables|Default|SetIsRight false)
  (CallFunction|FireBurst))

(event Collision|EventActorBeginOverlap
  (params (OtherActor :type Actor%20Object%20Reference))
  (bind _returnvalue (Transformation|GetActorRightVector))
  (|CallParentFunction OtherActor)
  (if (Actor|ActorHasTag OtherActor "Lateral")
    (if (Variables|Default|GetIsRight)
      (Variables|Default|SetIsRight false)
      (Variables|Default|SetMovementVector (* _returnvalue "0.000000,-1.000000,0.000000"))
      (Variables|Default|SetDelayShoot (- (Variables|Default|GetDelayShoot) 0.1))
      (else
        (Variables|Default|SetIsRight true)
        (Variables|Default|SetMovementVector _returnvalue)))))

(event EventTick
  (params (DeltaSeconds :type Float%20%28single-precision%29))
  (CallFunction|Move DeltaSeconds))

(fn ConstructionScript
  (|CallParentFunction))

(fn Fire
  (|CallParentFunction))